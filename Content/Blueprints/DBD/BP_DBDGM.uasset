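; Game mode for an asymmetric killer-versus-runners multiplayer game that assigns each joining player a role.
; In HandleStartingNewPlayer, the first player is stored as Killer and possesses a BP_Killer; while that reference stays valid, later players get a BP_Runner.
; Each pawn spawns at the player start named for its role.
; A random role assignment is sketched but unwired, and BeginPlay only calls CreateWidget.
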(event EventBeginPlay
  (UserInterface|CreateWidget 0))

(event EventHandleStartingNewPlayer
  (params (NewPlayer :type Player%20Controller%20Object%20Reference))
  (|CallParentFunction NewPlayer)
  (Utilities|IsValid (Variables|Default|GetKiller)
    (:Is%20Valid
      (bind _returnvalue (Game|SpawnActorfromClass "/Game/Characters/BP_Runner.BP_Runner_C" (Transformation|GetActorTransform (Class|GameModeBase|FindPlayerStart 0 "Runner")) "Undefined" "MultiplyWithRoot" 0 0))
      (Pawn|Possess NewPlayer _returnvalue))
    (:Is%20Not%20Valid
      (bind _output_get (Variables|Default|SetKiller NewPlayer))
      (bind _returnvalue_2 (Game|SpawnActorfromClass "/Game/Characters/BP_Killer.BP_Killer_C" (Transformation|GetActorTransform (Class|GameModeBase|FindPlayerStart 0 "Killer")) "Undefined" "MultiplyWithRoot" 0 0))
      (Pawn|Possess _output_get _returnvalue_2))))

(fn ConstructionScript)