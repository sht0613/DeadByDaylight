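; BP_Weapon is a melee weapon actor that a character carries and swings to deal damage.
; AttachToChar stores the character, turns off physics on the weapon and snaps it to a socket on the character's mesh.
; DoAttack plays a sword montage, while DoDamage box-traces between two weapon sockets, ignoring the wielder, with persistent debug drawing.
; DoDamage applies fixed damage to the first hit only, returning immediately afterward.
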(event EventBeginPlay)

(event Collision|EventActorBeginOverlap
  (params (OtherActor :type Actor%20Object%20Reference)))

(event EventTick
  (params (DeltaSeconds :type Float%20%28single-precision%29)))

(fn ConstructionScript)

(fn AttachtoChar
  (params (Character :type Character%20Object%20Reference))
  (bind _output_get (Variables|Default|SetCharacter Character))
  (Physics|SetSimulatePhysics (Variables|Default|GetWeapon) false)
  (Transformation|AttachComponentToComponent (Variables|/Script/Engine.Character|GetMesh _output_get) (Variables|Default|GetSocket%20Name) "SnapToTarget" "SnapToTarget" "KeepWorld" true)
  (return true))

(fn DoAttack
  (Animation|PlayAnimMontage (Variables|Default|GetCharacter) "/Game/Animation/AttacknGrab/SwordAttack/Sword_Attack.Sword_Attack" 1.0 "None")
  (return false))

(fn DoDamage
  (bind _weapon (Variables|Default|GetWeapon))
  (bind _outhits (Class|KismetSystemLibrary|BoxTraceMultiforObjects (Transformation|GetSocketLocation _weapon "UP") (Transformation|GetSocketLocation _weapon "Down") "1.000000,1.000000,1.000000" "0, 0, 0" (Utilities|Array|MakeArray "ObjectTypeQuery1" "ObjectTypeQuery2" "ObjectTypeQuery3" "ObjectTypeQuery4" "ObjectTypeQuery5" "ObjectTypeQuery6") false (Utilities|Array|MakeArray (Variables|Default|GetCharacter)) "Persistent" true))
  (for _array_element _outhits
    (Game|Damage|ApplyDamage (.HitActor (Collision|BreakHitResult _array_element)) 1e+01 (Pawn|GetController (Variables|Default|GetCharacter)) self)
    (return true)))